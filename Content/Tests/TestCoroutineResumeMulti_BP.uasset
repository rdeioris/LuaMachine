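; Functional test that checks LuaValueResumeMulti can resume a Lua coroutine with multiple arguments and return multiple values.
; StartTest runs the TestCoroutines code asset in LuaTestState, then resumes global coro5 repeatedly through a Sequence.
; It checks the success flag and selected returned values, plus the first result's length.
; A final resume without arguments must return false, and any mismatch fails the test.
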(event EventStartTest
  (Class|LuaBlueprintFunctionLibrary|LuaRunCodeAsset "/LuaMachine/LuaTestState.LuaTestState_C" "/LuaMachine/Code/TestCoroutines.TestCoroutines")
  (bind _returnvalue (Class|LuaBlueprintFunctionLibrary|LuaGetGlobal "/LuaMachine/LuaTestState.LuaTestState_C" "coro5"))
  (Utilities|FlowControl|Sequence
    (:then_0
      (bind _returnvalue_2 (Class|LuaBlueprintFunctionLibrary|LuaValueResumeMulti _returnvalue (Utilities|Array|MakeArray (Class|LuaBlueprintFunctionLibrary|LuaCreateInteger 2) (Class|LuaBlueprintFunctionLibrary|LuaCreateInteger 3) (Class|LuaBlueprintFunctionLibrary|LuaCreateInteger 4))))
      (if (not (== (Utilities|Array|Length _returnvalue_2) 4))
        (Class|FunctionalTest|FinishTest "Failed" "return values must be 4")))
    (:then_1
      (if (not (Class|LuaBlueprintFunctionLibrary|ToBoolean(LuaValue) (Utilities|Array|Get(acopy) _returnvalue_2)))
        (Class|FunctionalTest|FinishTest "Failed" "value is not true")))
    (:then_2
      (if (not (== (Class|LuaBlueprintFunctionLibrary|ToInteger(LuaValue) (Utilities|Array|Get(acopy) _returnvalue_2 3)) 20))
        (Class|FunctionalTest|FinishTest "Failed" "value is not 20")))
    (:then_3
      (bind _returnvalue_3 (Class|LuaBlueprintFunctionLibrary|LuaValueResumeMulti _returnvalue (Utilities|Array|MakeArray (Class|LuaBlueprintFunctionLibrary|LuaCreateInteger 7) (Class|LuaBlueprintFunctionLibrary|LuaCreateInteger 8) (Class|LuaBlueprintFunctionLibrary|LuaCreateInteger 9))))
      (if (== (Class|LuaBlueprintFunctionLibrary|ToInteger(LuaValue) (Utilities|Array|Get(acopy) _returnvalue_3 3)) 9000)
        (if (not (== (Class|LuaBlueprintFunctionLibrary|ToInteger(LuaValue) (Utilities|Array|Get(acopy) _returnvalue_3 4)) 17222630))
          (Class|FunctionalTest|FinishTest "Failed" "value is not 17222630"))
        (else
          (Class|FunctionalTest|FinishTest "Failed" "value is not 9000"))))
    (:then_4
      (bind _returnvalue_4 (Class|LuaBlueprintFunctionLibrary|LuaValueResumeMulti _returnvalue (Utilities|Array|MakeArray (Class|LuaBlueprintFunctionLibrary|LuaCreateInteger 10) (Class|LuaBlueprintFunctionLibrary|LuaCreateInteger 20) (Class|LuaBlueprintFunctionLibrary|LuaCreateInteger 30))))
      (if (not (Class|LuaBlueprintFunctionLibrary|ToBoolean(LuaValue) (Utilities|Array|Get(acopy) _returnvalue_4)))
        (Class|FunctionalTest|FinishTest "Failed" "value is not true")))
    (:then_5
      (if (not (== (Class|LuaBlueprintFunctionLibrary|ToInteger(LuaValue) (Utilities|Array|Get(acopy) _returnvalue_4 3)) 3))
        (Class|FunctionalTest|FinishTest "Failed" "value is not 3")))
    (:then_6
      (bind _returnvalue_5 (Class|LuaBlueprintFunctionLibrary|LuaValueResumeMulti _returnvalue))
      (if (Class|LuaBlueprintFunctionLibrary|ToBoolean(LuaValue) (Utilities|Array|Get(acopy) _returnvalue_5))
        (Class|FunctionalTest|FinishTest "Failed" "value is not false")))
    (:then_7
      (Class|FunctionalTest|FinishTest "Succeeded"))))

(fn ConstructionScript)